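; BP_Wall is a wall tile Blueprint that switches between a standing wall and a broken, floor-height state.
; It sets its type to Wall on BeginPlay, then checks its floor type every Tick.
; A BrokenWallFloor floor type resets it to unit scale with type None; any other value stretches it vertically and sets it to Wall.
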(event `self.ReceiveBeginPlay`
  (`parent.ReceiveBeginPlay`)
  (`self.SetType` "Wall"))

(event `self.ReceiveTick`
  (params (DeltaSeconds :type "Float (single-precision)"))
  (if (`|EnumEquality` (`self.m_FloorType`) "BrokenWallFloor")
    (`self.SetActorRelativeScale3D` (1.0 1.0 1.0))
    (`self.SetType` "None")
    (else
      (`self.SetActorRelativeScale3D` (1.0 1.0 5.0))
      (`self.SetType` "Wall"))))

(fn `UserConstructionScript`
  (`parent.UserConstructionScript`))