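; Player pawn for an RTS-style game, providing camera control, unit selection, NPC orders, spawning on random floor actors, and pause.
; Axis inputs pan with zoom-scaled speed, zoom within height limits and yaw while middle-click is held.
; Left-click traces to select NPCs or interactables, while dragging spawns a selection box.
; Right-click traces under the cursor to give selected controllable NPCs attack, follow, interact or move directives.
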(event `SpawnNPC`
  (params (Type :type String))
  (set `/Game/UI/WBP_Player.IsSpawningNPC` false (`self.RefToWidgetBP`))
  (switch `string` Type
    (:`Default`
      (`self.SpawnCharacter` "/Game/Blueprints/NPC/BP_Volunteer.BP_Volunteer_C" :!label _label))
    (:`Agent`
      (`self.SpawnCharacter` "/Game/Blueprints/NPC/BP_Agent.BP_Agent_C"))
    (:`Researcher`
      (`self.SpawnCharacter` "/Game/Blueprints/NPC/BP_Researcher.BP_Researcher_C"))
    (:`Volunteer`
      (goto _label))))

(event `InputAxis|Scroll`
  (params (AxisValue :type "Float (single-precision)"))
  (bind (_returnvalue_x _returnvalue_y _returnvalue_z) (`KismetMathLibrary.BreakVector` (`self.K2_GetActorLocation`)))
  ;[1 1 1] Map Movement (Translation)
  (`self.K2_SetActorLocation` (`KismetMathLibrary.MakeVector` _returnvalue_x _returnvalue_y (`KismetMathLibrary.FMin` (`KismetMathLibrary.FMax` (+ _returnvalue_z (* (* (* -1 AxisValue) (`self.DeltaTime`)) (`self.ScrollMagnitude`))) (`self.MinZoom`)) (`self.MaxZoom`)))))

(event `InputAxis|Forward`
  (params (AxisValue :type "Float (single-precision)"))
  ;[1 1 1] Map Movement (Translation)
  (`self.K2_SetActorLocation` (+ (`self.K2_GetActorLocation`) (* (* (`self.GetActorForwardVector`) AxisValue) (* (`self.DeltaTime`) (`self.MoveMagnitude`))))))

(event `ResetDrag`
  ;[1 1 1] Selection of objects
  (goto _label_2 :!via `Reset`))

(event `MouseDrag`
  ;[1 1 1] Selection of objects
  (if (not (== (`self.StartMousePosition`) (`self.FindMousePositionInWorld`) :`ErrorTolerance` 20.0))
    (`|ExecutionSequence`
      (:`then_0`
        (`/Engine/EditorBlueprintResources/StandardMacros.DoOnce` false :!label _label_2
          (:`Completed`
            (set `self.DragSuccess` true))))
      (:`then_1`
        (bind _outactors (`GameplayStatics.GetAllActorsOfClass` "/Game/Blueprints/Player/BP_SelectionBox.BP_SelectionBox_C"))
        (if (!= (`KismetArrayLibrary.Array_Length` _outactors) 1)
          (for _array_element _outactors
            (`self.K2_DestroyActor` _array_element))
          (`|SpawnActorFromClass` "/Game/Blueprints/Player/BP_SelectionBox.BP_SelectionBox_C" (`KismetMathLibrary.MakeTransform` (`self.StartMousePosition`)) "AlwaysSpawn" "OverrideRootScale" null null))))
    (else
      (set `self.DragSuccess` false))))

(event `self.ReceiveBeginPlay`
  ;[1 1 1] Begin play
  (bind _returnvalue (`|CreateWidget` "/Game/UI/WBP_Player.WBP_Player_C" (`GameplayStatics.GetPlayerController` 0)))
  (bind _output_get (set `self.RefToWidgetBP` _returnvalue))
  (`UserWidget.AddToViewport` _output_get 0))

(event `InputAction|LeftClick`
  (params (Key :type "Key Structure"))
  ;[1 1 1] Selection of objects
  (:`Pressed`
    (if (`self.HoveringButton`)
      (set `self.LeftClickPressed` true)
      (else
        (set `self.LeftClickPressed` true)
        (set `self.StartMousePosition` (`self.FindMousePositionInWorld`)))))
  (:`Released`
    (set `self.LeftClickPressed` false)
    (`self.ResetDrag`)
    (if (not (`self.DragSuccess`))
      (bind _outactors (`GameplayStatics.GetAllActorsOfClass` "/Script/ProjectImpetus.Tile3D"))
      (bind _outhit (`KismetSystemLibrary.LineTraceSingle` (`SceneComponent.K2_GetComponentLocation` (`self.Camera`)) (`self.FindMousePositionInWorld`) "TraceTypeQuery1" false _outactors))
      (bind (_bblockinghit _binitialoverlap _time _distance _location _impactpoint _normal _impactnormal _physmat _hitactor) (`GameplayStatics.BreakHitResult` _outhit))
      (`/Engine/EditorBlueprintResources/StandardMacros.IsValid` _hitactor
        (:`Is Valid`
          (cast `NPC` _hitactor
            (:`then`
              _)
            (:`CastFailed`
              (cast `/Game/Blueprints/Interactables/BP_BaseInteractable` _hitactor)))
          (`self.SelectActor` _hitactor)
          (`self.GetSelectedActors`))))))

(event `InputAxis|Right`
  (params (AxisValue :type "Float (single-precision)"))
  ;[1 1 1] Map Movement (Translation)
  (`self.K2_SetActorLocation` (+ (`self.K2_GetActorLocation`) (* (* (`self.GetActorRightVector`) AxisValue) (* (`self.DeltaTime`) (`self.MoveMagnitude`))))))

(event `MiddleClickHeld`
  ;[1 1 1] Map Movement (Rotation)
  (set `self.ZRotation` (+ (`self.ZRotation`) (* (* (`self.GetInputAxisKeyValue`) (`self.DeltaTime`)) (`self.RotateMagnitude`)))))

(event `InputAction|RightClick`
  (params (Key :type "Key Structure"))
  ;[1 1 1] Set directive for all selected NPC characters
  (:`Released`
    (bind _returnvalue (`self.GetSelectedActors`))
    (for _array_element _returnvalue
      (bind _asnpc (cast `NPC` _array_element))
      (bind _returnvalue_2 (`NPC.IsControllable` _asnpc))
      (if _returnvalue_2
        (`/Engine/EditorBlueprintResources/StandardMacros.IsValid` _asnpc
          (:`Is Valid`
            (bind (_success _outputdirective _hitactor) (`self.Set Directive`))
            (if _success
              (`NPC.SetDirective` _asnpc (cast `Directive` _outputdirective))
              (`NPC.SetFocus` _asnpc _hitactor))))))))

(event `self.ReceiveTick`
  (params (DeltaSeconds :type "Float (single-precision)"))
  (bind (_returnvalue_x _returnvalue_y _returnvalue_z) (`KismetMathLibrary.BreakVector` (`self.K2_GetActorLocation`)))
  ;[1 1 1] Tick Event
  (`|ExecutionSequence`
    (:`then_0`
      (set `self.DeltaTime` DeltaSeconds)
      ;;[1 1 1] Scale move speed to current zoom
      (set `self.MoveMagnitude` (`KismetMathLibrary.FMax` (* (`self.MaxMoveMagnitude`) (/ _returnvalue_z (`self.MaxZoom`))) (`self.MinMoveMagnitude`))))
    (:`then_1`
      (if (`self.MiddleClickPressed`)
        (`self.MiddleClickHeld`)))
    (:`then_2`
      (`self.UpdateRotation`))
    (:`then_3`
      (if (and (`self.LeftClickPressed`) (not (`self.HoveringButton`)))
        (`self.MouseDrag`)))))

(event `InputAction|MiddleClick`
  (params (Key :type "Key Structure"))
  ;[1 1 1] Map Movement (Rotation)
  (:`Pressed`
    (set `self.MiddleClickPressed` true))
  (:`Released`
    (set `self.MiddleClickPressed` false)))

(event `Key|AnyKey`
  (params (Key :type "Key Structure"))
  (:`Pressed`
    (set `self.CurrentKeyPressed` (`KismetInputLibrary.Key_GetDisplayName` Key)))
  (:`Released`
    (set `self.CurrentKeyPressed` "")))

(event `UpdateRotation`
  (bind (_returnvalue_roll _returnvalue_pitch) (`KismetMathLibrary.BreakRotator` (`self.K2_GetActorRotation`)))
  ;[1 1 1] Map Movement (Rotation)
  (`self.K2_SetActorRotation` (`KismetMathLibrary.MakeRotator` _returnvalue_roll _returnvalue_pitch (`self.ZRotation`))))

(event `InputAction|Pause` :paused true
  (params (Key :type "Key Structure"))
  (bind _returnvalue (not (`self.Paused`)))
  ;[1 1 1] Pause game
  (:`Released`
    (`GameplayStatics.SetGamePaused` _returnvalue)
    (set `self.Paused` _returnvalue)))

(fn `GetBoxMax`
  (returns (Max :type "Vector Structure"))
  (locals (Corner1 :type "Vector2D Structure") (Corner2 :type "Vector2D Structure") (Corner3 :type "Vector2D Structure") (Corner4 :type "Vector2D Structure"))
  (bind (_returnvalue_x _returnvalue_y) (`KismetMathLibrary.BreakVector` (`self.FindMousePositionInWorld`)))
  (bind (_startmouseposition_x _startmouseposition_y) (`KismetMathLibrary.BreakVector` (`self.StartMousePosition`)))
  (bind (_corner1_x _corner1_y) (`KismetMathLibrary.BreakVector2D` (`local.Corner1`)))
  (bind (_corner2_x _corner2_y) (`KismetMathLibrary.BreakVector2D` (`local.Corner2`)))
  (bind (_corner3_x _corner3_y) (`KismetMathLibrary.BreakVector2D` (`local.Corner3`)))
  (bind (_corner4_x _corner4_y) (`KismetMathLibrary.BreakVector2D` (`local.Corner4`)))
  (bind (_returnvalue_x_2 _returnvalue_y_2) (`KismetMathLibrary.BreakVector2D` (`KismetMathLibrary.MakeVector2D` (`KismetMathLibrary.FMax` (`KismetMathLibrary.FMax` _corner1_x _corner2_x) (`KismetMathLibrary.FMax` _corner3_x _corner4_x)) (`KismetMathLibrary.FMax` (`KismetMathLibrary.FMax` _corner1_y _corner2_y) (`KismetMathLibrary.FMax` _corner3_y _corner4_y)))))
  (set `local.Corner1` (`KismetMathLibrary.MakeVector2D` _startmouseposition_x _startmouseposition_y))
  (set `local.Corner2` (`KismetMathLibrary.MakeVector2D` _returnvalue_x _returnvalue_y))
  (set `local.Corner3` (`KismetMathLibrary.MakeVector2D` _returnvalue_x _startmouseposition_y))
  (set `local.Corner4` (`KismetMathLibrary.MakeVector2D` _startmouseposition_x _returnvalue_y))
  (return (`KismetMathLibrary.MakeVector` _returnvalue_x_2 _returnvalue_y_2)))

(fn `GetBoxMin`
  (returns (Min :type "Vector Structure"))
  (locals (Corner1 :type "Vector2D Structure") (Corner2 :type "Vector2D Structure") (Corner3 :type "Vector2D Structure") (Corner4 :type "Vector2D Structure"))
  (bind (_returnvalue_x _returnvalue_y) (`KismetMathLibrary.BreakVector` (`self.FindMousePositionInWorld`)))
  (bind (_startmouseposition_x _startmouseposition_y) (`KismetMathLibrary.BreakVector` (`self.StartMousePosition`)))
  (bind (_corner3_x _corner3_y) (`KismetMathLibrary.BreakVector2D` (`local.Corner3`)))
  (bind (_corner4_x _corner4_y) (`KismetMathLibrary.BreakVector2D` (`local.Corner4`)))
  (bind (_corner1_x _corner1_y) (`KismetMathLibrary.BreakVector2D` (`local.Corner1`)))
  (bind (_corner2_x _corner2_y) (`KismetMathLibrary.BreakVector2D` (`local.Corner2`)))
  (bind (_returnvalue_x_2 _returnvalue_y_2) (`KismetMathLibrary.BreakVector2D` (`KismetMathLibrary.MakeVector2D` (`KismetMathLibrary.FMin` (`KismetMathLibrary.FMin` _corner1_x _corner2_x) (`KismetMathLibrary.FMin` _corner3_x _corner4_x)) (`KismetMathLibrary.FMin` (`KismetMathLibrary.FMin` _corner1_y _corner2_y) (`KismetMathLibrary.FMin` _corner3_y _corner4_y)))))
  (set `local.Corner1` (`KismetMathLibrary.MakeVector2D` _startmouseposition_x _startmouseposition_y))
  (set `local.Corner2` (`KismetMathLibrary.MakeVector2D` _returnvalue_x _returnvalue_y))
  (set `local.Corner3` (`KismetMathLibrary.MakeVector2D` _returnvalue_x _startmouseposition_y))
  (set `local.Corner4` (`KismetMathLibrary.MakeVector2D` _startmouseposition_x _returnvalue_y))
  (return (`KismetMathLibrary.MakeVector` _returnvalue_x_2 _returnvalue_y_2)))

(fn `GetSelectionBoxCentroidPos`
  (returns (Loc :type "Vector Structure"))
  (return (/ (+ (`self.StartMousePosition`) (`self.FindMousePositionInWorld`)) 2.0)))

(fn `GetSelectionBoxHeight`
  (returns (Height :type "Float (double-precision)"))
  (bind (_returnvalue_x _returnvalue_y) (`KismetMathLibrary.BreakVector` (`self.FindMousePositionInWorld`)))
  (bind (_startmouseposition_x _startmouseposition_y) (`KismetMathLibrary.BreakVector` (`self.StartMousePosition`)))
  (return (- _returnvalue_y _startmouseposition_y)))

(fn `GetSelectionBoxWidth`
  (returns (Width :type "Float (double-precision)"))
  (bind _returnvalue_x (`KismetMathLibrary.BreakVector` (`self.FindMousePositionInWorld`)))
  (bind _startmouseposition_x (`KismetMathLibrary.BreakVector` (`self.StartMousePosition`)))
  (return (- _returnvalue_x _startmouseposition_x)))

(fn `Set Directive`
  (returns (Success :type Boolean) (OutputDirective :type Byte) (HitActor :type "Actor Object Reference"))
  (locals (Directive :type "Directive Enum" :default "MoveHere") (Focus :type "Actor Object Reference"))
  ;[1 1 1] Set directive based on what was clicked
  (set `local.Directive` "DoNothing")
  (bind _returnvalue (`self.GetSelectedActors`))
  (bind _outhit (`KismetSystemLibrary.LineTraceSingle` (`SceneComponent.K2_GetComponentLocation` (`self.Camera`)) (`self.FindMousePositionInWorld`) "TraceTypeQuery1" false _returnvalue))
  (bind (_bblockinghit _binitialoverlap _time _distance _location _impactpoint _normal _impactnormal _physmat _hitactor) (`GameplayStatics.BreakHitResult` _outhit))
  (`/Engine/EditorBlueprintResources/StandardMacros.IsValid` _hitactor
    (:`Is Valid`
      (set `local.Focus` _hitactor)
      (`|ExecutionSequence`
        (:`then_0`
          (bind _asnpc (cast `NPC` _hitactor))
          (if (`NPC.m_Threat` _asnpc)
            (bind _output_get (set `local.Directive` "AttackThis"))
            (return true _output_get (`local.Focus`))
            (else
              (bind _output_get_2 (set `local.Directive` "FollowThis"))
              (return true _output_get_2 (`local.Focus`)))))
        (:`then_1`
          (cast `Interactable` _hitactor)
          (bind _output_get_3 (set `local.Directive` "InteractThis"))
          (return true _output_get_3 (`local.Focus`)))
        (:`then_2`
          (cast `Tile3D` _hitactor
            (:`then`
              (bind _output_get_4 (set `local.Directive` "MoveHere"))
              (return true _output_get_4 (`local.Focus`)))
            (:`CastFailed`
              (return false (`local.Directive`) (`local.Focus`)))))))
    (:`Is Not Valid`
      (return false (`local.Directive`) (`local.Focus`)))))

(fn `SpawnCharacter`
  (params (ActorToSpawn :type "Actor Class Reference"))
  (bind _outactors (`GameplayStatics.GetAllActorsOfClass` "/Game/Blueprints/Tile/BP_Floor.BP_Floor_C"))
  (bind (_returnvalue_x _returnvalue_y) (`KismetMathLibrary.BreakVector` (`self.K2_GetActorLocation` (`KismetArrayLibrary.Array_Random` _outactors))))
  (`|SpawnActorFromClass` ActorToSpawn (`KismetMathLibrary.MakeTransform` (`KismetMathLibrary.MakeVector` _returnvalue_x _returnvalue_y)) "AlwaysSpawn" "OverrideRootScale" null null))

(fn `SwitchToIsometric`
  (`SceneComponent.K2_SetRelativeRotation` (`self.Camera`) (struct :`Pitch` -45.0) false false)
  (set `self.TopDown` false))

(fn `SwitchToTopDown`
  (`SceneComponent.K2_SetRelativeRotation` (`self.Camera`) (struct :`Pitch` -90.0) false false)
  (set `self.TopDown` true))

(fn `UserConstructionScript`)