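; Drag-selection box actor that lets the player select BP_BaseNPC units while left click is held.
; Each tick it moves to and resizes its collision box and cube visual from the player's selection box centroid, width and height.
; NPCs are found by testing every one's XY location against the player's box bounds, not by overlap events, and get an outline material while inside.
; On release it passes them to the player, resets their materials and destroys itself.
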(event `TrackOverlappingActors`
  (bind _playerref (`self.PlayerRef`))
  (bind _overlappedactors (`self.OverlappedActors`))
  ;[1 1 1] Keep track of overlapped actors
  (bind _outactors (`GameplayStatics.GetAllActorsOfClass` "/Game/Blueprints/NPC/BP_BaseNPC.BP_BaseNPC_C"))
  (for _array_element _outactors
    (bind _max (`/Game/Blueprints/Player/BP_Player.GetBoxMax` _playerref))
    (bind _min (`/Game/Blueprints/Player/BP_Player.GetBoxMin` _playerref))
    (bind (_returnvalue_x _returnvalue_y) (`KismetMathLibrary.BreakVector` (`self.K2_GetActorLocation` _array_element)))
    (if (and (and (<= _returnvalue_x (.x _max)) (<= _returnvalue_y (.y _max))) (and (>= _returnvalue_x (.x _min)) (>= _returnvalue_y (.y _min))))
      (bind _returnvalue (`KismetArrayLibrary.Array_Contains` _overlappedactors _array_element))
      (if (not _returnvalue)
        (`KismetArrayLibrary.Array_Add` _overlappedactors _array_element)
        (`PrimitiveComponent.SetMaterial` (`Character.Mesh` _array_element) 0 "/Game/Materials/M_NPC_Outline.M_NPC_Outline"))
      (elif _returnvalue
        (`KismetArrayLibrary.Array_RemoveItem` _overlappedactors _array_element)
        (`/Game/Blueprints/NPC/BP_BaseNPC.ResetMaterial` _array_element)))))

(event `self.ReceiveBeginPlay`
  ;[1 1 1] Begin play
  (`self.SetActorHiddenInGame` false)
  (bind _asbp_player (cast `/Game/Blueprints/Player/BP_Player` (`GameplayStatics.GetPlayerCharacter` 0)))
  (set `self.PlayerRef` _asbp_player))

(event `self.ReceiveTick`
  (params (DeltaSeconds :type "Float (single-precision)"))
  (bind _playerref (`self.PlayerRef`))
  (bind _cube (`self.Cube`))
  (bind (_returnvalue_x _returnvalue_y _returnvalue_z) (`KismetMathLibrary.BreakVector` (`SceneComponent.K2_GetComponentScale` _cube)))
  ;[1 1 1] Set box extents, visual and overlapping box
  (if (`/Game/Blueprints/Player/BP_Player.LeftClickPressed` (`self.PlayerRef`))
    (`self.TrackOverlappingActors`)
    (bind _loc (`/Game/Blueprints/Player/BP_Player.GetSelectionBoxCentroidPos` _playerref))
    (`self.K2_SetActorLocation` _loc)
    (bind _asbox_collision (cast `BoxComponent` (`self.CollisionComponent`)))
    (bind _width (`/Game/Blueprints/Player/BP_Player.GetSelectionBoxWidth` _playerref))
    (bind _height (`/Game/Blueprints/Player/BP_Player.GetSelectionBoxHeight` _playerref))
    (bind (_boxextent_x _boxextent_y _boxextent_z) (`KismetMathLibrary.BreakVector` (`BoxComponent.BoxExtent` _asbox_collision)))
    (bind _returnvalue (`KismetMathLibrary.MakeVector` (/ _width 2.0) (/ _height 2.0) _boxextent_z))
    (`BoxComponent.SetBoxExtent` _asbox_collision _returnvalue true)
    (bind (_returnvalue_x_2 _returnvalue_y_2) (`KismetMathLibrary.BreakVector` (/ _returnvalue 100.0)))
    (`SceneComponent.SetWorldScale3D` _cube (`KismetMathLibrary.MakeVector` (* _returnvalue_x_2 2.0) (* _returnvalue_y_2 2.0) _returnvalue_z))
    (else
      (`self.Kill`))))

(event `Kill`
  ;[1 1 1] Kill event
  (`PlayerCharacter.AddSelectedActors` (`self.PlayerRef`) (`self.OverlappedActors`))
  (for _array_element (`self.OverlappedActors`)
    (bind _asbp_base_npc (cast `/Game/Blueprints/NPC/BP_BaseNPC` _array_element))
    (`/Game/Blueprints/NPC/BP_BaseNPC.ResetMaterial` _asbp_base_npc))
  (`self.K2_DestroyActor`))

(fn `UserConstructionScript`)