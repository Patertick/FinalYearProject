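; Base NPC actor that shows its threat status by switching its mesh between threat and passive materials.
; BeginPlay requires a base Material in slot 0, then applies the material matching MThreat.
; Tick compares MThreat to OldThreatDesignation, which is never updated after BeginPlay, so any difference reapplies the material every frame.
; A SceneCaptureComponent2D limited to the NPC's own components captures on TakeScreenshot.
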(event `self.ReceiveBeginPlay`
  (bind _asmaterial (cast `Material` (`PrimitiveComponent.GetMaterial` (`self.Mesh`) 0)))
  (set `self.DefaultMaterial` _asmaterial)
  (bind _output_get (set `self.OldThreatDesignation` (`self.m_Threat`)))
  (if _output_get
    (set `self.DefaultMaterial` "/Game/Materials/M_NPC_Threat.M_NPC_Threat")
    (`self.ResetMaterial`)
    (else
      (set `self.DefaultMaterial` "/Game/Materials/M_NPC_Passive.M_NPC_Passive")
      (`self.ResetMaterial`))))

(event `self.ReceiveTick`
  (params (DeltaSeconds :type "Float (single-precision)"))
  (bind _m_threat (`self.m_Threat`))
  (if (!= _m_threat (`self.OldThreatDesignation`))
    (if _m_threat
      (set `self.DefaultMaterial` "/Game/Materials/M_NPC_Threat.M_NPC_Threat")
      (`self.ResetMaterial`)
      (else
        (set `self.DefaultMaterial` "/Game/Materials/M_NPC_Passive.M_NPC_Passive")
        (`self.ResetMaterial`)))))

(fn `ResetMaterial`
  (`PrimitiveComponent.SetMaterial` (`self.Mesh`) 0 (`self.DefaultMaterial`)))

(fn `TakeScreenshot`
  (`SceneCaptureComponent2D.CaptureScene` (`self.SceneCaptureComponent2D`)))

(fn `UserConstructionScript`
  (`SceneCaptureComponent.ShowOnlyActorComponents` (`self.SceneCaptureComponent2D`) self true))