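; BP_BaseInteractable is a base interactable actor that shows an outline material while flagged as seen and can capture an image of itself.
; BeginPlay caches the mesh's slot 0 material, only if it casts to Material.
; Tick sets either the outline or cached material every frame, based on MIsSeen.
; Construction limits the SceneCaptureComponent2D to this actor and its child actors, and TakeScreenshot triggers the capture on demand.
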(event `self.ReceiveBeginPlay`
  (bind _asmaterial (cast `Material` (`PrimitiveComponent.GetMaterial` (`self.m_Mesh`) 0)))
  (set `self.DefaultMaterial` _asmaterial))

(event `self.ReceiveTick`
  (params (DeltaSeconds :type "Float (single-precision)"))
  (if (`self.m_IsSeen`)
    (`PrimitiveComponent.SetMaterial` (`self.m_Mesh`) 0 "/Game/Materials/M_StaticMesh_Outline.M_StaticMesh_Outline")
    (else
      (`self.ResetMaterial`))))

(fn `ResetMaterial`
  (`PrimitiveComponent.SetMaterial` (`self.m_Mesh`) 0 (`self.DefaultMaterial`)))

(fn `TakeScreenshot`
  (`SceneCaptureComponent2D.CaptureScene` (`self.SceneCaptureComponent2D`)))

(fn `UserConstructionScript`
  (`SceneCaptureComponent.ShowOnlyActorComponents` (`self.SceneCaptureComponent2D`) self true))